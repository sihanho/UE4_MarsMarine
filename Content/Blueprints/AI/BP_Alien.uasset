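; BP_Alien is a spider-like enemy AI that chases the player and dies when damage drains its health.
; BeginPlay re-issues AIMoveTo toward the player controller after a short delay while alive.
; Tick pauses movement for an attack montage, but CanAttack requires IsAttacking both false and true, so it never fires; DamagePlayer has no caller here.
; Death disables movement and collision, credits BP_Marine's kill, notifies BP_NewGameMode, then destroys the actor.
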(event `self.ReceiveBeginPlay`
  (if (`self.IsAline`) :!label _label
    (`|AIMoveTo` self (0.0 0.0 0.0) (`GameplayStatics.GetPlayerController` 0)
      (:`OnSuccess`
        _)
      (:`OnFail`
        _))
    (`KismetSystemLibrary.Delay` 0.2)
    (goto _label)))

(event `self.ReceiveTick`
  (params (DeltaSeconds :type "Float (single-precision)"))
  (if (`self.CanAttack`)
    (`self.DeactivateAIMovement`)
    (`|PlayMontage` (`self.Mesh`) "/Game/Characters/Enemy_Great_Spider/Animations/SpiderAttack1.SpiderAttack1"
      (:`OnCompleted`
        (`self.ActivateAIMovement`)))))

(event `self.ReceiveAnyDamage`
  (params (Damage :type "Float (single-precision)") (DamageType :type "DamageType Object Reference") (InstigatedBy :type "Controller Object Reference") (DamageCauser :type "Actor Object Reference"))
  (if (`self.IsAline`)
    (bind _health (`self.DecreaseHealth` Damage))
    (if (== _health 0.0)
      (`self.KillAI`)
      (`KismetSystemLibrary.Delay` 3.0)
      (`self.K2_DestroyActor`))))

(fn `ActivateAIMovement`
  (`ActorComponent.Activate` (`self.CharacterMovement`) false))

(fn `CanAttack`
  (returns (ReturnValue :type Boolean))
  (return (and (`self.Is Within Attack Range`) (not (`self.IsAttacking`)) (`self.IsAttacking`))))

(fn `DamagePlayer`
  (locals (DamagePerHit :type "Float (double-precision)" :default 15.0))
  (if (`self.IsAline`)
    (`GameplayStatics.ApplyDamage` (`GameplayStatics.GetPlayerCharacter` 0) (`local.DamagePerHit`))))

(fn `DeactivateAIMovement`
  (bind _charactermovement (`self.CharacterMovement`))
  (`MovementComponent.StopMovementImmediately` _charactermovement)
  (`ActorComponent.Deactivate` _charactermovement))

(fn `DecreaseHealth`
  (params (B :type "Float (double-precision)"))
  (returns (Health :type "Float (double-precision)"))
  (bind _output_get (set `self.Health` (`KismetMathLibrary.FClamp` (- (`self.Health`) B) 0.0 100.0)))
  (return _output_get))

(fn `Is Within Attack Range`
  (returns (ReturnValue :type Boolean))
  (locals (AttackRange :type "Float (double-precision)" :default 150.0))
  (return (< (`self.GetDistanceTo` self (`GameplayStatics.GetPlayerCharacter` 0)) (`local.AttackRange`))))

(fn `IsAline`
  (returns (IsAlive :type Boolean))
  (return (not (`self.Dead`))))

(fn `IsAttacking`
  (returns (ReturnValue :type Boolean))
  (return (`AnimInstance.Montage_IsPlaying` (`SkeletalMeshComponent.GetAnimInstance` (`self.Mesh`)) "/Game/Characters/Enemy_Great_Spider/Animations/SpiderAttack1.SpiderAttack1")))

(fn `KillAI`
  (set `self.Dead` true)
  (`self.DeactivateAIMovement`)
  (`self.SetActorEnableCollision` false)
  (bind _asbp_marine (cast `/Game/Blueprints/Pawns/BP_Marine` (`GameplayStatics.GetPlayerCharacter` 0)))
  (`/Game/Blueprints/Pawns/BP_Marine.IncreaseKills` _asbp_marine)
  (bind _asbp_new_game_mode (cast `/Game/Blueprints/GameMode/BP_NewGameMode` (`GameplayStatics.GetGameMode`)))
  (`/Game/Blueprints/GameMode/BP_NewGameMode.RegisterAlienDeath` _asbp_new_game_mode self))

(fn `UserConstructionScript`)