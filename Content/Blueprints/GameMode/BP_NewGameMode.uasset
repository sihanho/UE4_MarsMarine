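; BP_NewGameMode is a game mode that spawns endless waves of BP_Alien enemies and tracks the living ones.
; After a short delay on BeginPlay, it increments the wave counter and starts a looping timer that spawns one alien per tick at a random TargetPoint.
; Spawned aliens join the Aliens array, RegisterAlienDeath removes them, and Tick prints the live count.
; No wave end or timer stop is present.
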(event `SpawnWave`
  (`self.SpawnAlien`))

(event `self.ReceiveBeginPlay`
  (`KismetSystemLibrary.Delay` 2.0)
  ;[1 1 1] has loop call function
  (`self.SetupNewWave`))

(event `self.ReceiveTick`
  (params (DeltaSeconds :type "Float (single-precision)"))
  (`KismetSystemLibrary.PrintString` (`KismetStringLibrary.Conv_IntToString` (`KismetArrayLibrary.Array_Length` (`self.Aliens`)))))

(fn `GetRandomSpawnPoint`
  (returns (Actor_TargetPoint :type "TargetPoint Object Reference"))
  (bind _outactors (`GameplayStatics.GetAllActorsOfClass` "/Script/Engine.TargetPoint"))
  (return (`|GetArrayItem` _outactors (`KismetMathLibrary.RandomIntegerInRange` 0 (`KismetArrayLibrary.Array_LastIndex` _outactors)))))

(fn `RegisterAlienDeath`
  (params (Alien :type "/Game/Blueprints/AI/BP_Alien Object Reference (by ref)"))
  (`KismetArrayLibrary.Array_RemoveItem` (`self.Aliens`) Alien))

(fn `SetupNewWave`
  (`/Engine/EditorBlueprintResources/StandardMacros.IncrementInt` (`self.CurrentWave`)
    (:`  `
      (`KismetSystemLibrary.K2_SetTimer` null "SpawnWave" 1.0 true))))

(fn `SpawnAlien`
  (bind _actor_targetpoint (`self.GetRandomSpawnPoint`))
  (`/Engine/EditorBlueprintResources/StandardMacros.IsValid` _actor_targetpoint
    (:`Is Valid`
      (bind _returnvalue (`|SpawnActorFromClass` "/Game/Blueprints/AI/BP_Alien.BP_Alien_C" (`self.GetTransform` _actor_targetpoint) "Undefined" "OverrideRootScale" null null))
      (`/Engine/EditorBlueprintResources/StandardMacros.IsValid` _returnvalue
        (:`Is Valid`
          (`KismetArrayLibrary.Array_Add` (`self.Aliens`) _returnvalue))))))

(fn `UserConstructionScript`)